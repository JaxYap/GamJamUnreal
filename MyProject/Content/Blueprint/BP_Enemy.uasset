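; Patrolling AI enemy that walks a looping waypoint route, chases players it sees, investigates noises and damages what its capsule hits.
; PawnSensing events recolor the spotlight as an alert indicator and trigger a move to the pawn or sound.
; A DoOnce gates the switch to sprinting, and retriggerable delays reset it and resume walking patrol once sensing events stop.
; A random navigable-point move exists but is never called.
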(event `self.ReceiveBeginPlay`
  (`self.PatrolEnemy`))

(event `PatrolEnemy`
  ;[1 1 1] Patrol Around Waypoints
  (`LightComponent.SetLightColor` (`self.SpotLight`) (struct :`R` 1.0 :`G` 1.0 :`B` 1.0 :`A` 1.0) true)
  (set `CharacterMovementComponent.MaxWalkSpeed` 130.0 (`self.CharacterMovement`))
  (`|AIMoveTo` self (`|GetArrayItem` (`self.Waypoints`) (`self.CurrentLocation`)) null
    (:`OnSuccess`
      (`self.PatrolEnemy`)
      (`/Engine/EditorBlueprintResources/StandardMacros.IncrementInt` (`self.CurrentLocation`)
        (:`  `
          (if (== (`self.CurrentLocation`) (`KismetArrayLibrary.Array_Length` (`self.Waypoints`)))
            (set `self.CurrentLocation` 0)))))))

(event `MoveToRandomLocation`
  ;[1 1 1] Move to Random Location
  (bind _randomlocation (`NavigationSystemV1.K2_GetRandomLocationInNavigableRadius` (`self.K2_GetActorLocation`) 500.0 null null))
  (`|AIMoveTo` self _randomlocation null))

(event `CanSprintAgain`
  ;[1 1 1] Enemy Detection
  (goto _label :!via `Reset`))

(event `self.PawnSensing.OnSeePawn`
  (params (Pawn :type "Pawn Object Reference"))
  ;[1 1 1] Enemy Detection
  (`LightComponent.SetLightColor` (`self.SpotLight`) (struct :`R` 1.0 :`G` 0.008924 :`A` 1.0) true)
  (`KismetSystemLibrary.PrintString` "I SEE YOU!!")
  (`|ExecutionSequence`
    (:`then_0`
      (`/Engine/EditorBlueprintResources/StandardMacros.DoOnce` false :!label _label
        (:`Completed`
          (`SkeletalMeshComponent.PlayAnimation` (`self.Mesh`) "/Game/Characters/Mannequins/Animations/Quinn/MF_Run_Fwd.MF_Run_Fwd" true)
          (set `CharacterMovementComponent.MaxWalkSpeed` 600.0 (`self.CharacterMovement`)))))
    (:`then_1`
      (`|AIMoveTo` self (0.0 0.0 0.0) Pawn
        (:`then`
          (`KismetSystemLibrary.RetriggerableDelay` 2.0)
          (`self.CanSprintAgain`)
          (`SkeletalMeshComponent.PlayAnimation` (`self.Mesh`) "/Game/Characters/Mannequins/Animations/Quinn/MF_Walk_Fwd.MF_Walk_Fwd" true)
          (set `CharacterMovementComponent.MaxWalkSpeed` 130.0 (`self.CharacterMovement`))
          (`self.PatrolEnemy`))))))

(event `self.PawnSensing.OnHearNoise`
  (params (Instigator :type "Pawn Object Reference") (Location :type "Vector Structure (by ref)") (Volume :type "Float (single-precision)"))
  ;[1 1 1] Enemy Sound Detection
  (`LightComponent.SetLightColor` (`self.SpotLight`) (struct :`R` 1.0 :`G` 0.940307 :`A` 1.0) true)
  (`KismetSystemLibrary.PrintString` "I can hear you!")
  (`|ExecutionSequence`
    (:`then_0`
      (goto _label))
    (:`then_1`
      (`|AIMoveTo` self Location null
        (:`then`
          (`KismetSystemLibrary.RetriggerableDelay` 2.0)
          (`self.CanSprintAgain`)
          (`SkeletalMeshComponent.PlayAnimation` (`self.Mesh`) "/Game/Characters/Mannequins/Animations/Quinn/MF_Walk_Fwd.MF_Walk_Fwd" true)
          (set `CharacterMovementComponent.MaxWalkSpeed` 130.0 (`self.CharacterMovement`))
          (`self.PatrolEnemy`))))))

(event `self.CapsuleComponent.OnComponentHit`
  (params (HitComponent :type "PrimitiveComponent Object Reference") (OtherActor :type "Actor Object Reference") (OtherComp :type "PrimitiveComponent Object Reference") (NormalImpulse :type "Vector Structure") (Hit :type "HitResult Structure (by ref)"))
  ;[1 1 1] Damage Player
  (`GameplayStatics.ApplyDamage` OtherActor 1.0 null self)
  (`self.PatrolEnemy`))

(fn `UserConstructionScript`)